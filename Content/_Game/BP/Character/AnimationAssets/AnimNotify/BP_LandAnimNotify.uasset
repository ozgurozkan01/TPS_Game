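; BP_LandAnimNotify is an animation notify that plays a surface-specific landing sound for a ShooterCharacter.
; When received, it casts the mesh owner to ShooterCharacter and, if its TracerComponent is valid, reads the surface type from it.
; A switch maps metal, stone, tile, grass or water to a land sound, defaulting to tile, and plays it at the character's location.
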(fn `Received_Notify`
  (params (MeshComp :type "SkeletalMeshComponent Object Reference") (Animation :type "AnimSequenceBase Object Reference") (EventReference :type "AnimNotifyEventReference Structure (by ref)"))
  (returns (ReturnValue :type Boolean))
  (locals (LandSound :type "SoundBase Object Reference"))
  (bind _asshooter_character (cast `ShooterCharacter` (`ActorComponent.GetOwner` MeshComp)))
  (bind _tracercomponent (`ShooterCharacter.TracerComponent` _asshooter_character))
  (`/Engine/EditorBlueprintResources/StandardMacros.IsValid` _tracercomponent
    (:`Is Valid`
      (bind _returnvalue (`TracerComponent.GetSurfaceType` _tracercomponent))
      (switch `EPhysicalSurface` _returnvalue
        (:`SurfaceType_Default`
          (set `local.LandSound` "/Game/_Game/BP/Character/Sounds/SoundCue/Land_Tile.Land_Tile"))
        (:`SurfaceType1`
          (set `local.LandSound` "/Game/_Game/BP/Character/Sounds/SoundCue/Land_Metal.Land_Metal"))
        (:`SurfaceType2`
          (set `local.LandSound` "/Game/_Game/BP/Character/Sounds/SoundCue/Land_Stone.Land_Stone"))
        (:`SurfaceType3`
          (set `local.LandSound` "/Game/_Game/BP/Character/Sounds/SoundCue/Land_Tile.Land_Tile"))
        (:`SurfaceType4`
          (set `local.LandSound` "/Game/_Game/BP/Character/Sounds/SoundCue/Land_Grass.Land_Grass"))
        (:`SurfaceType5`
          (set `local.LandSound` "/Game/_Game/BP/Character/Sounds/SoundCue/Land_Water.Land_Water")))
      (`GameplayStatics.PlaySoundAtLocation` (`local.LandSound`) (`Actor.K2_GetActorLocation` _asshooter_character) (struct) 1.0 1.0 0.0 null null null null)
      (return false))))