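; Anim notify that plays surface-dependent footstep sounds and Niagara effects for BP_ShooterCharacter animations.
; It gets the surface type from the character's TracerComponent, then picks a matching sound and particle system, falling back to wood sound and dirt particles.
; Both spawn at the configured socket on the mesh, with ShouldPlaySound gating only the sound.
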(fn `Received_Notify`
  (params (MeshComp :type "SkeletalMeshComponent Object Reference") (Animation :type "AnimSequenceBase Object Reference") (EventReference :type "AnimNotifyEventReference Structure (by ref)"))
  (returns (ReturnValue :type Boolean))
  (locals (FootstepSound :type "SoundBase Object Reference" :default "/Script/Engine.SoundWave'/Game/_Game/BP/Character/Sounds/SoundWave/Footstep_Wood.Footstep_Wood'") (FootstepNiagaraSystem :type "NiagaraSystem Object Reference" :default "/Script/Niagara.NiagaraSystem'/Game/A_Surface_Footstep/Niagara_FX/ParticleSystems/PSN_Dirt_Surface.PSN_Dirt_Surface'"))
  (bind _returnvalue (`SceneComponent.GetSocketLocation` MeshComp (`self.SocketNameOnBone`)))
  (bind _asbp_shooter_character (cast `/Game/_Game/BP/Character/BP_ShooterCharacter` (`ActorComponent.GetOwner` MeshComp)))
  (bind _tracercomponent (`ShooterCharacter.TracerComponent` _asbp_shooter_character))
  (`/Engine/EditorBlueprintResources/StandardMacros.IsValid` _tracercomponent
    (:`Is Valid`
      (bind _returnvalue_2 (`TracerComponent.GetSurfaceType` _tracercomponent))
      (switch `EPhysicalSurface` _returnvalue_2
        (:`SurfaceType_Default`
          (set `local.FootstepSound` "/Game/_Game/BP/Character/Sounds/SoundWave/Footstep_Wood.Footstep_Wood")
          (set `local.FootstepNiagaraSystem` "/Game/A_Surface_Footstep/Niagara_FX/ParticleSystems/PSN_Dirt_Surface.PSN_Dirt_Surface"))
        (:`SurfaceType1`
          (set `local.FootstepSound` "/Game/_Game/BP/Character/Sounds/SoundCue/Footstep_Metal_Cue.Footstep_Metal_Cue")
          (set `local.FootstepNiagaraSystem` "/Game/A_Surface_Footstep/Niagara_FX/ParticleSystems/PSN_General1_Surface.PSN_General1_Surface"))
        (:`SurfaceType2`
          (set `local.FootstepSound` "/Game/_Game/BP/Character/Sounds/SoundCue/Footstep_Stone.Footstep_Stone")
          (set `local.FootstepNiagaraSystem` "/Game/A_Surface_Footstep/Niagara_FX/ParticleSystems/PSN_Gravel_Surface.PSN_Gravel_Surface"))
        (:`SurfaceType3`
          (set `local.FootstepSound` "/Game/_Game/BP/Character/Sounds/SoundCue/Footstep_Tile.Footstep_Tile")
          (set `local.FootstepNiagaraSystem` "/Game/A_Surface_Footstep/Niagara_FX/ParticleSystems/PSN_General2_Surface.PSN_General2_Surface"))
        (:`SurfaceType4`
          (set `local.FootstepSound` "/Game/_Game/BP/Character/Sounds/SoundCue/Footstep_Grass_Cue.Footstep_Grass_Cue")
          (set `local.FootstepNiagaraSystem` "/Game/A_Surface_Footstep/Niagara_FX/ParticleSystems/PSN_Grass_Surface.PSN_Grass_Surface"))
        (:`SurfaceType5`
          (set `local.FootstepSound` "/Game/_Game/BP/Character/Sounds/SoundCue/Footstep_Water.Footstep_Water")
          (set `local.FootstepNiagaraSystem` "/Game/A_Surface_Footstep/Niagara_FX/ParticleSystems/PSN_WaterLight_Surface.PSN_WaterLight_Surface")))
      (if (`self.ShouldPlaySound`)
        (`GameplayStatics.PlaySoundAtLocation` (`local.FootstepSound`) _returnvalue (struct) 1.0 1.0 0.0 null null null null))
      (`NiagaraFunctionLibrary.SpawnSystemAtLocation` (`local.FootstepNiagaraSystem`) _returnvalue)
      (return false))))